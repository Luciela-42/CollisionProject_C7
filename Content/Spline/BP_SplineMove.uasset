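; BP_SplineMove is a Blueprint that moves a Cube back and forth along a Spline.
; From BeginPlay, a timeline value scaled by spline length gives the distance used to set the Cube's world location and rotation.
; When the timeline finishes, it flips IsMoveRight and re-runs the branch to play or reverse, producing a ping-pong motion.
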(event `self.ReceiveBeginPlay`
  (bind _spline (`self.Spline`))
  (if (`self.IsMoveRight`) :!label _label
    (bind (_direction _value) (`Timeline|타임라인_0` :!label _label_2)
      (:`Update`
        (bind _returnvalue (* _value (`SplineComponent.GetSplineLength` _spline)))
        (`SceneComponent.K2_SetWorldLocationAndRotation` (`self.Cube`) (`SplineComponent.GetLocationAtDistanceAlongSpline` _spline _returnvalue "World") (`SplineComponent.GetRotationAtDistanceAlongSpline` _spline _returnvalue "World") false false))
      (:`Finished`
        (set `self.IsMoveRight` (not (`self.IsMoveRight`)))
        (goto _label)))
    (else
      (goto _label_2 :!via `Reverse`))))

(fn `UserConstructionScript`)