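; Escalator floor actor that carries a cube step along a spline in a continuous loop.
; A fast repeating timer started on BeginPlay advances the distance by Speed and sets the cube's world location and rotation from the spline.
; At the spline's end the timer stops and cube collision is disabled briefly, then a delayed reset returns it to the start, re-enables collision and restarts movement.
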(event `self.ReceiveBeginPlay`
  (`KismetSystemLibrary.K2_SetTimer` null "MoveOnSpline" 0.01 true))

(fn `MoveOnSpline`
  (bind _escalatorspline (`self.EscalatorSpline`))
  (bind _distance (`self.Distance`))
  (set `self.Distance` (+ (`self.Distance`) (`self.Speed`)))
  (`SceneComponent.K2_SetWorldLocationAndRotation` (`self.Cube`) (`SplineComponent.GetLocationAtDistanceAlongSpline` _escalatorspline _distance "World") (`SplineComponent.GetRotationAtDistanceAlongSpline` _escalatorspline _distance "World") false false)
  (if (>= (`self.Distance`) (`SplineComponent.GetSplineLength` (`self.EscalatorSpline`)))
    (`KismetSystemLibrary.K2_ClearTimer` null "MoveOnSpline")
    (`self.SleepTime`)))

(fn `ResetPosition`
  (bind _escalatorspline (`self.EscalatorSpline`))
  (bind _cube (`self.Cube`))
  (bind _output_get (set `self.Distance` 0.0))
  (`SceneComponent.K2_SetWorldLocationAndRotation` _cube (`SplineComponent.GetLocationAtDistanceAlongSpline` _escalatorspline _output_get "World") (`SplineComponent.GetRotationAtDistanceAlongSpline` _escalatorspline _output_get "World") false false)
  (`PrimitiveComponent.SetCollisionEnabled` _cube "QueryAndPhysics")
  (`KismetSystemLibrary.K2_SetTimer` null "MoveOnSpline" 0.01 true))

(fn `SleepTime`
  (`PrimitiveComponent.SetCollisionEnabled` (`self.Cube`) "NoCollision")
  (`KismetSystemLibrary.K2_SetTimer` null "ResetPosition" 0.1))

(fn `UserConstructionScript`)