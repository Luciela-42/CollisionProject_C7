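; BP_Cannon is a cannon actor that fires bullets automatically at a fixed interval.
; BeginPlay starts a looping timer that calls the Shot function by name.
; Shot spawns an actor of the SpawnBullet class at the Arrow component's world transform.
; If the spawn succeeds, it plays a P_Explosion emitter at the ParticleSystem component's location and rotation as a firing effect.
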(event `self.ReceiveBeginPlay`
  (`KismetSystemLibrary.K2_SetTimer` null "Shot" 3.0 true))

(fn `Shot`
  (bind _particlesystem (`self.ParticleSystem`))
  (bind _returnvalue (`|SpawnActorFromClass` (`self.SpawnBullet`) (`SceneComponent.K2_GetComponentToWorld` (`self.Arrow`)) "Undefined" "OverrideRootScale" null null))
  (if (`KismetSystemLibrary.IsValid` _returnvalue)
    (`GameplayStatics.SpawnEmitterAtLocation` "/Game/StarterContent/Particles/P_Explosion.P_Explosion" (`SceneComponent.K2_GetComponentLocation` _particlesystem) (`SceneComponent.K2_GetComponentRotation` _particlesystem))))

(fn `UserConstructionScript`)